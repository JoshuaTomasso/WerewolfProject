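; Player state for a Werewolf-style social deduction game, handling each player's role reveal and night action.
; Client events show timed widgets for the role, with text from DT_Roles, and for werewolf partner names.
; Server_SubmitNightAction checks phase, alive status and prior submission, counts self or partner picks as errors, then sets NightTarget if the role's bCanActAtNight allows.
; RepNotifies on role, target and error count fire change dispatchers.
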(event Custom|Server_SubmitNightAction
  (params (AbilityTarget :type BP%20Player%20State%20Object%20Reference))
  ;[0.15 0.15 0.15 0.5] Submiting the Night Action
  (bind _asbp_game_state (Utilities|Casting|CastToBP_GameState (Game|GetGameState)))
  (if (Math|Boolean|ANDBoolean (Utilities|Enum|Equal(Enum) "NewEnumerator1" (Variables|/Game/Blueprints/Management/BP_GameState.BP_GameState_C|GetCurrentPhase _asbp_game_state)) (Variables|Default|GetbIsAlive self) (== (Variables|Default|GetbHasSubmittedNightAction) false) (Variables|BP_PlayerState_C|GetbIsAlive AbilityTarget))
    (if (or (== self AbilityTarget) (== (Variables|Default|GetWerewolfPartner) AbilityTarget))
      (Development|PrintString "Voted for Yourself or Your Partner" true true "(R=1.000000,G=0.000000,B=0.000000,A=1.000000)" 1e+02)
      (Math|Integer|IncrementInt (Variables|Default|GetVoteErrorCount%20))
      (else
        (switch Utilities|FlowControl|Switch|SwitchonE_Roles (Variables|Default|GetCurrentRole self)
          (:NewEnumerator0
            (bind _returnvalue (Utilities|GetDataTableRow "/Game/Blueprints/PlayerRoles/DT_Roles.DT_Roles" "Villager")
              (:then
                (if (.bcanactatnight _returnvalue)
                  (Variables|Default|SetNightTarget AbilityTarget)
                  (Variables|Default|SetbHasSubmittedNightAction true)))))
          (:NewEnumerator1
            (bind _returnvalue_2 (Utilities|GetDataTableRow "/Game/Blueprints/PlayerRoles/DT_Roles.DT_Roles" "Werewolf")
              (:then
                (if (.bcanactatnight _returnvalue_2)
                  (Variables|Default|SetNightTarget AbilityTarget)
                  (Variables|Default|SetbHasSubmittedNightAction true)))))
          (:NewEnumerator2
            (bind _returnvalue_3 (Utilities|GetDataTableRow "/Game/Blueprints/PlayerRoles/DT_Roles.DT_Roles" "Medic")
              (:then
                (if (.bcanactatnight _returnvalue_3)
                  (Variables|Default|SetNightTarget AbilityTarget)
                  (Variables|Default|SetbHasSubmittedNightAction true)))))
          (:NewEnumerator3
            (bind _returnvalue_4 (Utilities|GetDataTableRow "/Game/Blueprints/PlayerRoles/DT_Roles.DT_Roles" "Mayor")
              (:then
                (if (.bcanactatnight _returnvalue_4)
                  (Variables|Default|SetNightTarget AbilityTarget)
                  (Variables|Default|SetbHasSubmittedNightAction true)))))
          (:NewEnumerator4
            (bind _returnvalue_5 (Utilities|GetDataTableRow "/Game/Blueprints/PlayerRoles/DT_Roles.DT_Roles" "Seer")
              (:then
                (if (.bcanactatnight _returnvalue_5)
                  (Variables|Default|SetNightTarget AbilityTarget)
                  (Variables|Default|SetbHasSubmittedNightAction true))))))))))

(event Custom|Client_RevealWerewolfPartner
  (params (PartnerNames :type Text))
  ;[0.15 0.15 0.15 0.5] Show Werewolves Who Their Teammates Are
  (Utilities|FlowControl|Delay 5.0)
  (bind _returnvalue (UserInterface|CreateWidget "/Game/Widgets/WBP_WerewolfPartnerReveal.WBP_WerewolfPartnerReveal_C" (Game|GetPlayerController self)))
  (UserInterface|Viewport|AddtoViewport _returnvalue 0)
  (Variables|/Script/UMG.TextBlock|SetText (Variables|/Game/Widgets/WBP_WerewolfPartnerReveal.WBP_WerewolfPartnerReveal_C|GetWerewolfNames _returnvalue) PartnerNames)
  (Utilities|FlowControl|Delay (Variables|Default|GetDuration))
  (Widget|RemovefromParent _returnvalue))

(event Custom|Client_ReceiveRole
  (params (RoleToReaveal :type E_Roles%20Enum :default "NewEnumerator0"))
  ;[0.15 0.15 0.15 0.5] Show The Player Their Role And What Their Objective Is
  (bind _returnvalue (UserInterface|CreateWidget "/Game/Widgets/WBP_PlayerRoleDiscription.WBP_PlayerRoleDiscription_C" (Game|GetPlayerController self)))
  (UserInterface|Viewport|AddtoViewport _returnvalue 0)
  (switch Utilities|FlowControl|Switch|SwitchonE_Roles RoleToReaveal
    (:NewEnumerator0
      (bind _returnvalue_2 (Utilities|GetDataTableRow "/Game/Blueprints/PlayerRoles/DT_Roles.DT_Roles" "Villager")
        (:then
          (Variables|/Script/UMG.TextBlock|SetText (Variables|/Game/Widgets/WBP_PlayerRoleDiscription.WBP_PlayerRoleDiscription_C|GetRoleText _returnvalue) (.DisplayName (Utilities|Struct|BreakS_RoleInfo _returnvalue_2)))
          (Variables|/Script/UMG.TextBlock|SetText (Variables|/Game/Widgets/WBP_PlayerRoleDiscription.WBP_PlayerRoleDiscription_C|GetRoleDetails _returnvalue) (.Description (Utilities|Struct|BreakS_RoleInfo _returnvalue_2))))))
    (:NewEnumerator1
      (bind _returnvalue_3 (Utilities|GetDataTableRow "/Game/Blueprints/PlayerRoles/DT_Roles.DT_Roles" "Werewolf")
        (:then
          (Variables|/Script/UMG.TextBlock|SetText (Variables|/Game/Widgets/WBP_PlayerRoleDiscription.WBP_PlayerRoleDiscription_C|GetRoleText _returnvalue) (.DisplayName (Utilities|Struct|BreakS_RoleInfo _returnvalue_3)))
          (Variables|/Script/UMG.TextBlock|SetText (Variables|/Game/Widgets/WBP_PlayerRoleDiscription.WBP_PlayerRoleDiscription_C|GetRoleDetails _returnvalue) (.Description (Utilities|Struct|BreakS_RoleInfo _returnvalue_3))))))
    (:NewEnumerator2
      (bind _returnvalue_4 (Utilities|GetDataTableRow "/Game/Blueprints/PlayerRoles/DT_Roles.DT_Roles" "Medic")
        (:then
          (Variables|/Script/UMG.TextBlock|SetText (Variables|/Game/Widgets/WBP_PlayerRoleDiscription.WBP_PlayerRoleDiscription_C|GetRoleText _returnvalue) (.DisplayName (Utilities|Struct|BreakS_RoleInfo _returnvalue_4)))
          (Variables|/Script/UMG.TextBlock|SetText (Variables|/Game/Widgets/WBP_PlayerRoleDiscription.WBP_PlayerRoleDiscription_C|GetRoleDetails _returnvalue) (.Description (Utilities|Struct|BreakS_RoleInfo _returnvalue_4))))))
    (:NewEnumerator3
      (bind _returnvalue_5 (Utilities|GetDataTableRow "/Game/Blueprints/PlayerRoles/DT_Roles.DT_Roles" "Mayor")
        (:then
          (Variables|/Script/UMG.TextBlock|SetText (Variables|/Game/Widgets/WBP_PlayerRoleDiscription.WBP_PlayerRoleDiscription_C|GetRoleText _returnvalue) (.DisplayName (Utilities|Struct|BreakS_RoleInfo _returnvalue_5)))
          (Variables|/Script/UMG.TextBlock|SetText (Variables|/Game/Widgets/WBP_PlayerRoleDiscription.WBP_PlayerRoleDiscription_C|GetRoleDetails _returnvalue) (.Description (Utilities|Struct|BreakS_RoleInfo _returnvalue_5))))))
    (:NewEnumerator4
      (bind _returnvalue_6 (Utilities|GetDataTableRow "/Game/Blueprints/PlayerRoles/DT_Roles.DT_Roles" "Seer")
        (:then
          (Variables|/Script/UMG.TextBlock|SetText (Variables|/Game/Widgets/WBP_PlayerRoleDiscription.WBP_PlayerRoleDiscription_C|GetRoleText _returnvalue) (.DisplayName (Utilities|Struct|BreakS_RoleInfo _returnvalue_6)))
          (Variables|/Script/UMG.TextBlock|SetText (Variables|/Game/Widgets/WBP_PlayerRoleDiscription.WBP_PlayerRoleDiscription_C|GetRoleDetails _returnvalue) (.Description (Utilities|Struct|BreakS_RoleInfo _returnvalue_6)))))))
  (Utilities|FlowControl|Delay (Variables|Default|GetDuration))
  (Widget|RemovefromParent _returnvalue))

(event EventBeginPlay)

(event EventTick
  (params (DeltaSeconds :type Float%20%28single-precision%29)))

(fn ConstructionScript)

(fn OnRepNightTarget
  (Default|CallOnNightTargetChanged))

(fn OnRepCurrentRole
  (Default|CallOnRoleAssigned))

(fn OnRepVoteErrorCount
  (Default|CallOnVoteErrorChanged))