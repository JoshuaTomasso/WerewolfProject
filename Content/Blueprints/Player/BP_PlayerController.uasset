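; Player controller for a werewolf-style role game, handling the ready handshake and night-action targeting UI.
; On BeginPlay the local controller creates the phase timer and hidden targeting widgets and adds input mapping.
; Tick polls GameState, notifying GameMode through a server event once all expected players are present.
; Tick also toggles cursor and input mode by phase, showing targeting only for roles DT_Roles allows to act at night.
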(event Custom|Server_NotifyReady
  (bind _asbp_game_mode (Utilities|Casting|CastToBP_GameMode (Game|GetGameMode)))
  (Default|NotifyPlayerReady _asbp_game_mode self))

(event EventBeginPlay
  (bind _returnvalue (PlayerController|LocalPlayerSubsystems|GetEnhancedInputLocalPlayerSubsystem))
  (if (Pawn|IsLocalController self)
    (bind _returnvalue_2 (UserInterface|CreateWidget "/Game/Widgets/WBP_GamePhaseTimer.WBP_GamePhaseTimer_C" self))
    (UserInterface|Viewport|AddtoViewport _returnvalue_2 0)
    (bind _returnvalue_3 (UserInterface|CreateWidget "/Game/Widgets/WBP_NightActionTargeting.WBP_NightActionTargeting_C" self))
    (bind _output_get (Variables|Default|SetNightActionWidget _returnvalue_3))
    (UserInterface|Viewport|AddtoViewport _output_get 100)
    (Widget|SetVisibility _output_get "Collapsed")
    (Utilities|IsValid _returnvalue
      (:Is%20Valid
        (Input|AddMappingContext _returnvalue "/Game/Inputs/IMC_PlayerInputs.IMC_PlayerInputs" 0 "(bIgnoreAllPressedKeysUntilRelease=True,bForceImmediately=False,bNotifyUserSettings=False)"))
      (:Is%20Not%20Valid
        (Development|PrintString "No Valid Input System" true true "(R=1.000000,G=0.000000,B=0.000000,A=1.000000)" 0.5)))))

(event EventTick
  (params (DeltaSeconds :type Float%20%28single-precision%29))
  (bind _self self)
  (bind _self_2 self)
  ;[0.15 0.15 0.15 0.5] This is to show the player list for night abilities
  (if (Pawn|IsLocalController self)
    (Utilities|FlowControl|Sequence
      (:then_0
        (if (== (Variables|Default|GetbHasAckedReady) false)
          (bind _asbp_game_state (Utilities|Casting|CastToBP_GameState (Game|GetGameState)))
          (if (and (> (Variables|/Game/Blueprints/Management/BP_GameState.BP_GameState_C|GetExpectedPlayerCount _asbp_game_state) 0) (>= (Utilities|Array|Length (Variables|/Script/Engine.GameStateBase|GetPlayerArray _asbp_game_state)) (Variables|/Game/Blueprints/Management/BP_GameState.BP_GameState_C|GetExpectedPlayerCount _asbp_game_state)))
            (CallFunction|ServerNotifyReady)
            (Variables|Default|SetbHasAckedReady true))))
      (:then_1
        (bind _asbp_game_state_2 (Utilities|Casting|CastToBP_GameState (Game|GetGameState)))
        (if (and (Utilities|Enum|Equal(Enum) (Variables|/Game/Blueprints/Management/BP_GameState.BP_GameState_C|GetCurrentPhase _asbp_game_state_2) "NewEnumerator1") (Variables|Default|GetbHasAckedReady))
          (if (== (Variables|Default|GetbNightWidgetShown) false)
            (bind _asbp_player_state (Utilities|Casting|CastToBP_PlayerState (Variables|GetPlayerState self)))
            (Variables|Default|SetbShowMouseCursor _self true)
            (Input|SetInputModeGameandUI _self (Variables|Default|GetNightActionWidget) "DoNotLock" true false)
            (switch Utilities|FlowControl|Switch|SwitchonE_Roles (Variables|/Game/Blueprints/Player/BP_PlayerState.BP_PlayerState_C|GetCurrentRole _asbp_player_state)
              (:NewEnumerator0
                (bind _returnvalue (Utilities|GetDataTableRow "/Game/Blueprints/PlayerRoles/DT_Roles.DT_Roles" "Villager")
                  (:then
                    (if (.bcanactatnight _returnvalue)
                      (Widget|SetVisibility (Variables|Default|GetNightActionWidget) "Visible")
                      (Variables|Default|SetbNightWidgetShown true)))))
              (:NewEnumerator1
                (bind _returnvalue_2 (Utilities|GetDataTableRow "/Game/Blueprints/PlayerRoles/DT_Roles.DT_Roles" "Werewolf")
                  (:then
                    (if (.bcanactatnight _returnvalue_2)
                      (Widget|SetVisibility (Variables|Default|GetNightActionWidget) "Visible")
                      (Variables|Default|SetbNightWidgetShown true)))))
              (:NewEnumerator2
                (bind _returnvalue_3 (Utilities|GetDataTableRow "/Game/Blueprints/PlayerRoles/DT_Roles.DT_Roles" "Medic")
                  (:then
                    (if (.bcanactatnight _returnvalue_3)
                      (Widget|SetVisibility (Variables|Default|GetNightActionWidget) "Visible")
                      (Variables|Default|SetbNightWidgetShown true)))))
              (:NewEnumerator3
                (bind _returnvalue_4 (Utilities|GetDataTableRow "/Game/Blueprints/PlayerRoles/DT_Roles.DT_Roles" "Mayor")
                  (:then
                    (if (.bcanactatnight _returnvalue_4)
                      (Widget|SetVisibility (Variables|Default|GetNightActionWidget) "Visible")
                      (Variables|Default|SetbNightWidgetShown true)))))
              (:NewEnumerator4
                (bind _returnvalue_5 (Utilities|GetDataTableRow "/Game/Blueprints/PlayerRoles/DT_Roles.DT_Roles" "Seer")
                  (:then
                    (if (.bcanactatnight _returnvalue_5)
                      (Widget|SetVisibility (Variables|Default|GetNightActionWidget) "Visible")
                      (Variables|Default|SetbNightWidgetShown true)))))))
          (elif (Variables|Default|GetbNightWidgetShown)
            (Widget|SetVisibility (Variables|Default|GetNightActionWidget) "Collapsed")
            (Variables|Default|SetbNightWidgetShown false)
            (Variables|Default|SetbShowMouseCursor _self_2 false)
            (Input|SetInputModeGameOnly _self_2 false)))))))

(fn ConstructionScript)