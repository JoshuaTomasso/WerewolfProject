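; Game mode for a multiplayer Werewolf game, handling role assignment, phase flow and night kills.
; Once enough players report ready, it deals a shuffled, hard-coded four-role pool, reveals werewolf partners and starts Night.
; StartPhase writes phase timing to BP_GameState and sets a timer intended to cycle Night, Day and Voting.
; ResolveNightActions reads the first two werewolves' targets, skips protected players and picks randomly between differing targets.
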(event Custom|OnPhaseTimerComplete
  (bind _asbp_game_state (Utilities|Casting|CastToBP_GameState (Game|GetGameState)))
  (switch Utilities|FlowControl|Switch|SwitchonE_GamePhase (Variables|/Game/Blueprints/Management/BP_GameState.BP_GameState_C|GetCurrentPhase _asbp_game_state)
    (:NewEnumerator0
      (CallFunction|StartPhase "NewEnumerator1"))
    (:NewEnumerator1
      (CallFunction|ResolveNightActions)
      (CallFunction|StartPhase "NewEnumerator2"))
    (:NewEnumerator2
      (CallFunction|StartPhase "NewEnumerator3"))
    (:NewEnumerator3
      (CallFunction|StartPhase "NewEnumerator1"))))

(event EventBeginPlay
  (bind _asbp_game_state (Utilities|Casting|CastToBP_GameState (Game|GetGameState)))
  (Variables|/Game/Blueprints/Management/BP_GameState.BP_GameState_C|SetExpectedPlayerCount _asbp_game_state (Variables|Default|GetExpectedPlayerCount)))

(event EventTick
  (params (DeltaSeconds :type Float%20%28single-precision%29)))

(event EventPostLogin
  (params (NewPlayer :type Player%20Controller%20Object%20Reference)))

(fn ConstructionScript)

(fn AssignRoles
  (bind _werewolves (Variables|Default|GetWerewolves))
  (bind _werewolves_2 (Variables|Default|GetWerewolves))
  (bind _output (Utilities|Array|Get(acopy) _werewolves))
  (bind _output_2 (Utilities|Array|Get(acopy) _werewolves 1))
  (Utilities|Array|Clear (Variables|Default|GetPlayerStates))
  (for _array_element (Variables|/Script/Engine.GameStateBase|GetPlayerArray (Game|GetGameState))
    (bind _asbp_player_state (Utilities|Casting|CastToBP_PlayerState _array_element)
      (:then
        (Utilities|Array|Add (Variables|Default|GetPlayerStates) _asbp_player_state))
      (:CastFailed
        (Development|PrintString "Cast to BP_PlayerState: Failed" true true "(R=1.000000,G=0.000000,B=0.000000,A=1.000000)" 1e+02))))
  (Utilities|Array|Clear (Variables|Default|GetRolePool))
  (Utilities|Array|Add (Variables|Default|GetRolePool) "NewEnumerator1")
  (Utilities|Array|Add (Variables|Default|GetRolePool) "NewEnumerator1")
  (Utilities|Array|Add (Variables|Default|GetRolePool) "NewEnumerator2")
  (Utilities|Array|Add (Variables|Default|GetRolePool) "NewEnumerator4")
  (Utilities|Array|Shuffle (Variables|Default|GetRolePool))
  (for _index (range 0 (- (Utilities|Array|Length (Variables|Default|GetPlayerStates)) 1))
    (bind _output_get (Variables|/Game/Blueprints/Player/BP_PlayerState.BP_PlayerState_C|SetCurrentRole (Utilities|Array|Get(acopy) (Variables|Default|GetPlayerStates) _index) (Utilities|Array|Get(acopy) (Variables|Default|GetRolePool) _index)))
    (Default|ClientReceiveRole (Utilities|Array|Get(acopy) (Variables|Default|GetPlayerStates) _index) _output_get)
    (if (Utilities|Enum|Equal(Enum) _output_get (Variables|Default|GetWerewolfRole))
      (Utilities|Array|Add _werewolves (Utilities|Array|Get(acopy) (Variables|Default|GetPlayerStates) _index))
      (Variables|/Game/Blueprints/Player/BP_PlayerState.BP_PlayerState_C|SetWerewolfPartner _output _output_2)
      (if (> (Utilities|Array|Length _werewolves) 1)
        (Variables|/Game/Blueprints/Player/BP_PlayerState.BP_PlayerState_C|SetWerewolfPartner _output_2 _output))))
  (for _array_element_2 _werewolves_2
    (Variables|Default|SetPartnerNamesText "")
    (for _array_element_3 _werewolves_2
      (if (!= _array_element_2 _array_element_3)
        (if (Utilities|Text|TextIsEmpty (Variables|Default|GetPartnerNamesText))
          (Variables|Default|SetPartnerNamesText (|GenerictoText (PlayerState|GetPlayerName _array_element_3)))
          (else
            (Variables|Default|SetPartnerNamesText (|GenerictoText (Utilities|String|Append (Utilities|String|ToString(Text) (Variables|Default|GetPartnerNamesText)) ", " (PlayerState|GetPlayerName _array_element_3))))))))
    (Default|ClientRevealWerewolfPartner _array_element_2 (Variables|Default|GetPartnerNamesText)))
  (Utilities|Array|Clear (Variables|Default|GetWerewolfPacks))
  (for _index_2 (range 0 (- (Utilities|Array|Length (Variables|Default|GetWerewolves)) 1))
    (if (== (Math|Integer|%(Integer) _index_2 2) 0)
      (if (< (+ _index_2 1) (Utilities|Array|Length (Variables|Default|GetWerewolves)))
        (Utilities|Array|Add (Variables|Default|GetWerewolfPacks) (Utilities|Struct|MakeS_WerewolfPack (Utilities|Array|Get(acopy) (Variables|Default|GetWerewolves) _index_2) (Utilities|Array|Get(acopy) (Variables|Default|GetWerewolves) (+ _index_2 1))))
        (else
          (Utilities|Array|Add (Variables|Default|GetWerewolfPacks) (Utilities|Struct|MakeS_WerewolfPack (Utilities|Array|Get(acopy) (Variables|Default|GetWerewolves) _index_2))))))))

(fn StartPhase
  (params (NewPhase :type E_GamePhase%20Enum :default "NewEnumerator0"))
  (bind _returnvalue (Utilities|Time|GetGameTimeinSeconds))
  (bind _asbp_game_state (Utilities|Casting|CastToBP_GameState (Game|GetGameState)))
  (bind _output_get (Variables|/Game/Blueprints/Management/BP_GameState.BP_GameState_C|SetCurrentPhase _asbp_game_state NewPhase))
  (switch Utilities|FlowControl|Switch|SwitchonE_GamePhase _output_get
    (:NewEnumerator0
      (bind _output_get_2 (Variables|/Game/Blueprints/Management/BP_GameState.BP_GameState_C|SetPhaseTimeRemaining _asbp_game_state 0.0))
      (bind _output_get_3 (Variables|/Game/Blueprints/Management/BP_GameState.BP_GameState_C|SetPhaseDuration _asbp_game_state _output_get_2))
      (Variables|/Game/Blueprints/Management/BP_GameState.BP_GameState_C|SetPhaseEndTime _asbp_game_state (+ _output_get_3 _returnvalue)))
    (:NewEnumerator1
      (bind _output_get_4 (Variables|/Game/Blueprints/Management/BP_GameState.BP_GameState_C|SetPhaseTimeRemaining _asbp_game_state (Variables|Default|GetNightDuration)))
      (bind _output_get_5 (Variables|/Game/Blueprints/Management/BP_GameState.BP_GameState_C|SetPhaseDuration _asbp_game_state _output_get_4))
      (Variables|/Game/Blueprints/Management/BP_GameState.BP_GameState_C|SetPhaseEndTime _asbp_game_state (+ _output_get_5 _returnvalue))
      (for _array_element (Variables|Default|GetPlayerStates)
        (Variables|/Game/Blueprints/Player/BP_PlayerState.BP_PlayerState_C|SetbHasSubmittedNightAction _array_element false)
        (Variables|/Game/Blueprints/Player/BP_PlayerState.BP_PlayerState_C|SetNightTarget _array_element 0)))
    (:NewEnumerator2
      (bind _output_get_6 (Variables|/Game/Blueprints/Management/BP_GameState.BP_GameState_C|SetPhaseTimeRemaining _asbp_game_state (Variables|Default|GetDayDuration)))
      (bind _output_get_7 (Variables|/Game/Blueprints/Management/BP_GameState.BP_GameState_C|SetPhaseDuration _asbp_game_state _output_get_6))
      (Variables|/Game/Blueprints/Management/BP_GameState.BP_GameState_C|SetPhaseEndTime _asbp_game_state (+ _output_get_7 _returnvalue)))
    (:NewEnumerator3
      (bind _output_get_8 (Variables|/Game/Blueprints/Management/BP_GameState.BP_GameState_C|SetPhaseTimeRemaining _asbp_game_state (Variables|Default|GetVotingDuration)))
      (bind _output_get_9 (Variables|/Game/Blueprints/Management/BP_GameState.BP_GameState_C|SetPhaseDuration _asbp_game_state _output_get_8))
      (Variables|/Game/Blueprints/Management/BP_GameState.BP_GameState_C|SetPhaseEndTime _asbp_game_state (+ _output_get_9 _returnvalue))))
  (Utilities|Time|ClearandInvalidateTimerbyHandle (Variables|Default|GetPhaseTimerHandle))
  (bind _returnvalue_2 (Utilities|Time|SetTimerbyEvent (EventDispatchers|CreateEvent :!event Custom|OnPhaseTimerComplete) (Variables|/Game/Blueprints/Management/BP_GameState.BP_GameState_C|GetPhaseTimeRemaining _asbp_game_state)))
  (Variables|Default|SetPhaseTimerHandle _returnvalue_2))

(fn NotifyPlayerReady
  (params (Controller :type BP%20Player%20Controller%20Object%20Reference))
  (bind _readyplayercontrollers (Variables|Default|GetReadyPlayerControllers))
  (if (== (Utilities|Array|ContainsItem (Variables|Default|GetReadyPlayerControllers) Controller) false)
    (Utilities|Array|Add _readyplayercontrollers Controller)
    (if (and (>= (Utilities|Array|Length _readyplayercontrollers) (Variables|Default|GetExpectedPlayerCount)) (== (Variables|Default|GetbGameStarted) false))
      (bind _asbp_game_state (Utilities|Casting|CastToBP_GameState (Game|GetGameState)))
      (Default|MulticastSendFinalPlayerList _asbp_game_state)
      (CallFunction|AssignRoles)
      (CallFunction|StartPhase "NewEnumerator1")
      (Variables|Default|SetbGameStarted true))))

(fn ResolveNightActions
  (bind _werewolves (Variables|Default|GetWerewolves))
  (bind _werewolves_2 (Variables|Default|GetWerewolves))
  (bind _killtargetarray (Variables|Default|GetKillTargetArray))
  (Utilities|FlowControl|Sequence
    (:then_0
      (Utilities|IsValid (Variables|/Game/Blueprints/Player/BP_PlayerState.BP_PlayerState_C|GetNightTarget (Utilities|Array|Get(acopy) _werewolves_2))
        (:Is%20Valid
          (if (Variables|/Game/Blueprints/Player/BP_PlayerState.BP_PlayerState_C|GetbIsProtected (Variables|/Game/Blueprints/Player/BP_PlayerState.BP_PlayerState_C|GetNightTarget (Utilities|Array|Get(acopy) _werewolves_2)))
            (Development|PrintString "Player Is Protected" true true "(R=0.000000,G=1.000000,B=0.000000,A=1.000000)" 1e+02 :!label _label)
            (else
              (Variables|Default|SetbAValid true)
              (Utilities|Array|Add _killtargetarray (Variables|/Game/Blueprints/Player/BP_PlayerState.BP_PlayerState_C|GetNightTarget (Utilities|Array|Get(acopy) _werewolves_2))))))))
    (:then_1
      (Utilities|IsValid (Variables|/Game/Blueprints/Player/BP_PlayerState.BP_PlayerState_C|GetNightTarget (Utilities|Array|Get(acopy) _werewolves_2 1))
        (:Is%20Valid
          (if (Variables|/Game/Blueprints/Player/BP_PlayerState.BP_PlayerState_C|GetbIsProtected (Variables|/Game/Blueprints/Player/BP_PlayerState.BP_PlayerState_C|GetNightTarget (Utilities|Array|Get(acopy) _werewolves_2 1)))
            (goto _label)
            (else
              (Variables|Default|SetbBValid true)
              (Utilities|Array|Add _killtargetarray 0))))))
    (:then_2
      (if (and (Variables|Default|GetbAValid) (Variables|Default|GetbBValid))
        (if (== (Variables|/Game/Blueprints/Player/BP_PlayerState.BP_PlayerState_C|GetNightTarget (Utilities|Array|Get(acopy) _werewolves_2)) (Variables|/Game/Blueprints/Player/BP_PlayerState.BP_PlayerState_C|GetNightTarget (Utilities|Array|Get(acopy) _werewolves_2 1)))
          (Variables|Default|SetKillTarget (Utilities|Array|Get(acopy) (Variables|Default|GetKillTargetArray)))
          (else
            (Variables|Default|SetKillTarget (.OutItem (Utilities|Array|Random (Variables|Default|GetKillTargetArray))))))
        (elif (Variables|Default|GetbAValid)
          (Variables|Default|SetKillTarget (Variables|/Game/Blueprints/Player/BP_PlayerState.BP_PlayerState_C|GetNightTarget (Utilities|Array|Get(acopy) _werewolves_2)))
          (elif (Variables|Default|GetbBValid)
            (Variables|Default|SetKillTarget (Variables|/Game/Blueprints/Player/BP_PlayerState.BP_PlayerState_C|GetNightTarget (Utilities|Array|Get(acopy) _werewolves_2 1)))))))
    (:then_3
      (Utilities|IsValid (Variables|Default|GetKillTarget)
        (:Is%20Valid
          (Variables|/Game/Blueprints/Player/BP_PlayerState.BP_PlayerState_C|SetbIsAlive (Variables|Default|GetKillTarget) false)
          (Development|PrintString (Utilities|String|Append (PlayerState|GetPlayerName (Variables|Default|GetKillTarget)) " Has Died") true true "(R=1.000000,G=0.000000,B=0.000000,A=1.000000)" 1e+02))))
    (:then_4
      (Variables|/Game/Blueprints/Player/BP_PlayerState.BP_PlayerState_C|SetNightTarget (Utilities|Array|Get(acopy) _werewolves) 0)
      (Variables|/Game/Blueprints/Player/BP_PlayerState.BP_PlayerState_C|SetNightTarget (Utilities|Array|Get(acopy) _werewolves 1) 0))))